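; Actor component that lets an owner grab a physics primitive and pull it toward a target location set from outside.
; Grabbing backs up and overrides gravity, damping and Pawn collision, and releasing restores them.
; While holding, Tick applies a mass-independent force at the center of mass toward the target, with strength scaled by distance within clamped min/max ranges.
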(event `GrabComponent`
  (params (`Primitive Component` :type "PrimitiveComponent Object Reference"))
  (bind _attachedcomponent (`self.AttachedComponent`))
  (`/Engine/EditorBlueprintResources/StandardMacros.IsValid` `Primitive Component`
    (:`Is Valid`
      (`self.AttachedComponent`
        (:`then`
          (`self.ReleaseComponent`))
        (:`else`
          _))
      (set `self.AttachedComponent` `Primitive Component`)
      (`self.SetComponentTickEnabled` true)
      (set `self.BkpGravityEnabled` (`PrimitiveComponent.IsGravityEnabled` _attachedcomponent))
      (`PrimitiveComponent.SetEnableGravity` _attachedcomponent false)
      (set `self.BkpLinearDamping` (`PrimitiveComponent.GetLinearDamping` _attachedcomponent))
      (`PrimitiveComponent.SetLinearDamping` _attachedcomponent (`self.LinearDamping`))
      (set `self.BkpAngularDamping` (`PrimitiveComponent.GetAngularDamping` _attachedcomponent))
      (`PrimitiveComponent.SetAngularDamping` _attachedcomponent (`self.AngularDamping`))
      (set `self.BkpPawnCollision` (`PrimitiveComponent.GetCollisionResponseToChannel` _attachedcomponent "ECC_Pawn"))
      (`PrimitiveComponent.SetCollisionResponseToChannel` _attachedcomponent "ECC_Pawn" "ECR_Ignore"))))

(event `ReleaseComponent`
  (bind _attachedcomponent (`self.AttachedComponent`)
    (:`then`
      (`PrimitiveComponent.SetLinearDamping` _attachedcomponent (`self.BkpLinearDamping`))
      (`PrimitiveComponent.SetAngularDamping` _attachedcomponent (`self.BkpAngularDamping`))
      (`PrimitiveComponent.SetEnableGravity` _attachedcomponent (`self.BkpGravityEnabled`))
      (`PrimitiveComponent.SetCollisionResponseToChannel` _attachedcomponent "ECC_Pawn" (`self.BkpPawnCollision`))
      (set `self.AttachedComponent` null)
      (`self.SetComponentTickEnabled` false))
    (:`else`)))

(event `self.ReceiveTick`
  (params (DeltaSeconds :type "Float (single-precision)"))
  (bind _returnvalue (- (`self.TargetLocation`) (`PrimitiveComponent.GetCenterOfMass` (`self.AttachedComponent`) "None")))
  (`/Engine/EditorBlueprintResources/StandardMacros.IsValid` (`self.AttachedComponent`)
    (:`Is Valid`
      (`PrimitiveComponent.AddForce` (`self.AttachedComponent`) (* (`KismetMathLibrary.Normal` _returnvalue) (`KismetMathLibrary.MapRangeClamped` (`KismetMathLibrary.VSize` _returnvalue) (`self.MinStrengthDistance`) (`self.MaxStrengthDistance`) (`self.MinStrength`) (`self.MaxStrength`))) "None" true))))

(fn `SetTargetLocation`
  (params (TargetLocation :type "Vector Structure"))
  (set `self.TargetLocation` TargetLocation))