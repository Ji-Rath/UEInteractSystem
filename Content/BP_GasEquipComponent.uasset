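; BP_GasEquipComponent is an equip component that ties item equipping to the Gameplay Ability System.
; EquipItem calls the parent, then reads the owner's equipped item data from an instanced struct, but does nothing with it.
; The GiveAbility node that would set StoredAbility is disconnected, so equipping grants no ability.
; UnequipItem calls the parent and clears StoredAbility from the owner's Ability System Component.
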(event `self.EquipItem`
  (params (Item :type "ItemHandle Structure (by ref)"))
  (`parent.EquipItem` Item)
  (bind _value (`BlueprintInstancedStructLibrary.GetInstancedStructValue` (`.ItemData` (break `InventoryContents` (`/InteractionSystem/BFL_Inventory.TryGetEquippedItemData` (`self.GetOwner`)))))))

(event `self.UnequipItem`
  (`parent.UnequipItem`)
  (`AbilitySystemComponent.ClearAbility` (`AbilitySystemBlueprintLibrary.GetAbilitySystemComponent` (`self.GetOwner`)) (`self.StoredAbility`)))